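; BP_Interactable_CardReader is an interactable card reader that unlocks its linked door for characters holding an authorized keycard.
; Interact checks the character's Keycard and ReaderAvailable list, printing a failure message otherwise.
; Success fires once, calling the door's MulticastModifyVar and spawning a card that a timeline swipes from Start to End.
; A second timeline flies the card toward the character before destroying it; sound and hue-shift nodes are unconnected.
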(event EventBeginPlay
  (|CallParentFunction) ; This node is disabled and will not be called.\nDrag off pins to build functionality.
)

(event Collision|EventActorBeginOverlap
  (params (OtherActor :type Actor%20Object%20Reference))
  (|CallParentFunction OtherActor) ; This node is disabled and will not be called.\nDrag off pins to build functionality.
)

(event EventTick
  (params (DeltaSeconds :type Float%20%28single-precision%29))
  (|CallParentFunction DeltaSeconds) ; This node is disabled and will not be called.\nDrag off pins to build functionality.
)

(event EventInteract
  (params (CharRef :type Bp%20Char%20Master%20Object%20Reference))
  (Variables|Default|SetCharRef CharRef)
  (if (Variables|/Game/Framework/Blueprints/bp_char_master.bp_char_master_C|GetKeycard? (Variables|Default|GetCharRef))
    (bind _array_element (Utilities|Array|ForEachLoopwithBreak (Variables|/Game/Framework/Blueprints/bp_char_master.bp_char_master_C|GetReaderAvailable (Variables|Default|GetCharRef)) :!label _label)
      (:LoopBody
        (if (== _array_element self)
          (Variables|Default|SetAvailable? true)
          (goto _label Break)
          (else
            (Variables|Default|SetAvailable? false))))
      (:Completed
        (if (Variables|Default|GetAvailable?)
          (Utilities|FlowControl|DoOnce false
            (:Completed
              (Default|MulticastModifyVar (Variables|Default|GetDoorToOpen))
              (bind _returnvalue (Game|SpawnActorfromClass "/Game/Framework/Blueprints/Child/BP_Interactable_Card.BP_Interactable_Card_C" (Math|Transform|MakeTransform "0, 0, 0") "AdjustIfPossibleButAlwaysSpawn" 0 0))
              (bind _output_get (Variables|Default|SetSwipeCard _returnvalue))
              (Utilities|IsValid _output_get
                (:Is%20Valid
                  (Transformation|SetActorRotation _output_get (Math|Rotator|MakeRotator (.Roll (Math|Rotator|BreakRotator (Transformation|GetActorRotation _output_get))) (.Pitch (Math|Rotator|BreakRotator (Transformation|GetActorRotation _output_get))) (.Yaw (Math|Rotator|BreakRotator (Transformation|GetActorRotation)))))
                  (bind _lerpcard (Timeline|Lerp PlayFromStart)
                    (:Update
                      (Utilities|IsValid (Variables|/Game/Framework/Blueprints/Master/BP_Interactable_Master.BP_Interactable_Master_C|GetInteractable (Variables|Default|GetSwipeCard))
                        (:Is%20Valid
                          (Transformation|SetWorldLocation (Variables|/Game/Framework/Blueprints/Master/BP_Interactable_Master.BP_Interactable_Master_C|GetInteractable (Variables|Default|GetSwipeCard)) (Math|Vector|Lerp(Vector) (Transformation|GetWorldLocation (Variables|Default|GetStart)) (Transformation|GetWorldLocation (Variables|Default|GetEnd)) _lerpcard) false false))))
                    (:Finished
                      (Utilities|IsValid (Variables|Default|GetCharRef)
                        (:Is%20Valid
                          (bind _lerpreturn (Timeline|LerpReturn PlayFromStart)
                            (:Update
                              (Utilities|IsValid (Variables|Default|GetSwipeCard)
                                (:Is%20Valid
                                  (Collision|SetCollisionEnabled (Variables|/Game/Framework/Blueprints/Master/BP_Interactable_Master.BP_Interactable_Master_C|GetInteractable (Variables|Default|GetSwipeCard)) "NoCollision")
                                  (Transformation|SetActorLocation (Variables|Default|GetSwipeCard) (Math|Vector|Lerp(Vector) (Transformation|GetActorLocation (Variables|Default|GetSwipeCard)) (Math|Vector|MakeVector (.x (Transformation|GetActorLocation (Variables|Default|GetCharRef))) (.y (Transformation|GetActorLocation (Variables|Default|GetCharRef))) (+ (.z (Transformation|GetActorLocation (Variables|Default|GetCharRef))) 125.0)) _lerpreturn) false false))))
                            (:Finished
                              (Utilities|IsValid (Variables|Default|GetSwipeCard)
                                (:Is%20Valid
                                  (Actor|DestroyActor (Variables|Default|GetSwipeCard))))))))))))))
          (else
            (Development|PrintString "Unable to open." :!label _label_2)))))
    (else
      (goto _label_2))))

(fn ConstructionScript
  (|CallParentFunction))