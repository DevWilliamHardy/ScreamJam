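; Interactable vending machine that sells a single health can to the patient character for one coin.
; BeginPlay spawns the can inside; interacting with at least one coin spends it and spawns a coin at the slot, guarded by a DoOnce.
; Chained timelines slide the coin in, move and drop the can, and rotate a machine mesh part.
; After a short delay, the machine calls Interact on the can for that character.
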(event Custom|interact
  (params (CharRef :type Bp%20Char%20Master%20Object%20Reference))
  (bind _asbp_char_patient (Utilities|Casting|CastTobp_char_Patient CharRef))
  (Variables|Default|SetBP:_Char_Patient_Ref _asbp_char_patient)
  (if (>= (Variables|/Game/Framework/Blueprints/bp_char_Patient.bp_char_Patient_C|GetCoinCount _asbp_char_patient) 1)
    (Utilities|FlowControl|DoOnce false
      (:Completed
        (bind _returnvalue (Game|SpawnActorfromClass "/Game/Framework/Blueprints/Child/BP_Interactable_Coin.BP_Interactable_Coin_C" (Math|Transform|MakeTransform "0, 0, 0") "AlwaysSpawn" 0 0))
        (Variables|Default|SetCoinRef _returnvalue)
        (Variables|/Game/Framework/Blueprints/bp_char_Patient.bp_char_Patient_C|SetCoinCount (Variables|Default|GetBP:_Char_Patient_Ref) (- (Variables|/Game/Framework/Blueprints/bp_char_Patient.bp_char_Patient_C|GetCoinCount (Variables|Default|GetBP:_Char_Patient_Ref)) 1))
        (Transformation|AttachComponentToComponent (Variables|Default|GetCoinRef) (Variables|Default|GetCoinLocStart) "None" "SnapToTarget" "SnapToTarget" "SnapToTarget" true)
        (bind _lerpcoin (Timeline|lerp PlayFromStart)
          (:Update
            (Transformation|SetRelativeLocation (Variables|Default|GetCoinLocStart) (Math|Vector|Lerp(Vector) (Variables|Default|GetBaseStartLoc) (Variables|/Script/Engine.SceneComponent|GetRelativeLocation (Variables|Default|GetCoinLocEnd)) _lerpcoin) false false))
          (:Finished
            (bind _lerpcoin_2 (Timeline|LerpCan PlayFromStart)
              (:Update
                (Transformation|SetRelativeLocation (Variables|Default|GetCan%20Start) (Math|Vector|Lerp(Vector) (Variables|Default|GetBaseCanLoc) (Variables|Default|GetDesiredLocCan) _lerpcoin_2) false false))
              (:Finished
                (bind _lerpcoin_3 (Timeline|LerpDrop PlayFromStart)
                  (:Update
                    (Transformation|SetRelativeLocation (Variables|Default|GetCan%20Start) (Math|Vector|Lerp(Vector) (Variables|Default|GetDesiredLocCan) (Variables|Default|GetBaseVendCan) _lerpcoin_3) false false))
                  (:Finished
                    (bind _lerpcoin_4 (Timeline|Timeline_0 PlayFromStart)
                      (:Update
                        (Transformation|SetRelativeRotation (Variables|Default|GetVendingMachine__1__polySurface1) (Math|Rotator|Lerp(Rotator) (Variables|/Script/Engine.SceneComponent|GetRelativeRotation (Variables|Default|GetVendingMachine__1__polySurface1)) "0, 0,40.000000" _lerpcoin_4) false false))
                      (:Finished
                        (Utilities|FlowControl|Delay 0.75)
                        (CallFunction|Interact (Variables|Default|GetCanRef) (Variables|Default|GetBP:_Char_Patient_Ref))))))))))))))

(event EventBeginPlay
  (|CallParentFunction)
  (Variables|Default|SetBaseStartLoc (Variables|/Script/Engine.SceneComponent|GetRelativeLocation (Variables|Default|GetCoinLocStart)))
  (Variables|Default|SetBaseCanLoc (Variables|/Script/Engine.SceneComponent|GetRelativeLocation (Variables|Default|GetCan%20Start)))
  (bind _returnvalue (Game|SpawnActorfromClass "/Game/Framework/Blueprints/Child/BP_Interactable_Health_Can.BP_Interactable_Health_Can_C" (Math|Transform|MakeTransform "0, 0, 0") "AlwaysSpawn" 0 0))
  (bind _output_get (Variables|Default|SetCanRef _returnvalue))
  (Transformation|AttachComponentToComponent _output_get (Variables|Default|GetCan%20Start) "None" "SnapToTarget" "SnapToTarget" "SnapToTarget" true))

(event Collision|EventActorBeginOverlap
  (params (OtherActor :type Actor%20Object%20Reference))
  (|CallParentFunction OtherActor) ; This node is disabled and will not be called.\nDrag off pins to build functionality.
)

(event EventTick
  (params (DeltaSeconds :type Float%20%28single-precision%29))
  (|CallParentFunction DeltaSeconds))

(fn ConstructionScript
  (|CallParentFunction))