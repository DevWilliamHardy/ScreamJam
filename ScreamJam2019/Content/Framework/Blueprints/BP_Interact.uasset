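; BP_Interact provides the interaction function that lets a character use interactable objects in front of the camera.
; It sphere-traces a short distance from the follow camera along the control rotation on the Visibility channel, with debug drawing enabled.
; A hit BP_Interactable_Master receives Interact.
; If its item name is non-empty and the character is a bp_char_Patient, the item's name and icon go to that character's AddWidget.
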(fn FInteract
  (params (FollowCamera :type Scene%20Component%20Object%20Reference) (Character :type Bp%20Char%20Master%20Object%20Reference))
  (bind _returnvalue (Transformation|GetWorldLocation FollowCamera))
  (bind (_outhit _returnvalue_2) (Collision|SphereTraceByChannel _returnvalue (+ _returnvalue (* (Math|Vector|GetForwardVector (Pawn|GetControlRotation Character :!class /Script/Engine.Pawn)) 168.0)) 5.0 "TraceTypeQuery1" false 0 "ForDuration"))
  (if _returnvalue_2
    (bind _asbp_interactable_master (Utilities|Casting|CastToBP_Interactable_Master (.HitActor (Collision|BreakHitResult _outhit))))
    (Default|Interact _asbp_interactable_master Character)
    (if (not (Utilities|Enum|Equal(Enum) (Variables|/Game/Framework/Blueprints/Master/BP_Interactable_Master.BP_Interactable_Master_C|GetitemName _asbp_interactable_master) ""))
      (bind _asbp_char_patient (Utilities|Casting|CastTobp_char_Patient Character))
      (Utilities|IsValid _asbp_char_patient
        (:Is%20Valid
          (Default|AddWidget _asbp_char_patient (Variables|/Game/Framework/Blueprints/Master/BP_Interactable_Master.BP_Interactable_Master_C|GetitemName _asbp_interactable_master) (Variables|/Game/Framework/Blueprints/Master/BP_Interactable_Master.BP_Interactable_Master_C|GetitemImage _asbp_interactable_master)))))))