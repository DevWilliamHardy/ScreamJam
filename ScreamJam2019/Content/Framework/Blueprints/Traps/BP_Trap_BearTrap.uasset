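; Bear trap Blueprint that snaps shut and damages the first patient character to overlap its sphere.
; The overlap fires once, with no reset, then triggers the claws and requests damage through a server event.
; An authority-check function routes the snap to a multicast event, going through a server event on remotes.
; A timeline rotates both claws closed, each lerping from the other claw's current rotation.
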(event OnComponentBeginOverlap(Sphere)
  (params (OverlappedComponent :type Primitive%20Component%20Object%20Reference) (OtherActor :type Actor%20Object%20Reference) (OtherComp :type Primitive%20Component%20Object%20Reference) (OtherBodyIndex :type Integer) (bFromSweep :type Boolean) (SweepResult :type Hit%20Result%20Structure%20%28by%20ref%29))
  (bind _asbp_char_patient (Utilities|Casting|CastTobp_char_Patient OtherActor))
  (bind _output_get (Variables|Default|SetCharRef _asbp_char_patient))
  (Utilities|FlowControl|DoOnce false
    (:Completed
      (CallFunction|FCheckServer)
      (CallFunction|ServerApplyDamage _output_get 4e+01))))

(event Custom|server_ApplyDamage
  (params (DamagedActor :type Actor%20Object%20Reference) (BaseDamage :type Float%20%28single-precision%29))
  (Game|Damage|ApplyDamage DamagedActor BaseDamage 0 0))

(event Custom|multicast_claws
  (bind _lerp (Timeline|Lerp Play)
    (:Update
      (Transformation|SetRelativeRotation (Variables|Default|GetLeftClaw) (Math|Rotator|Lerp(Rotator) (Variables|/Script/Engine.SceneComponent|GetRelativeRotation (Variables|Default|GetRightClaw)) "-60.000000,0.000000, 0" _lerp) false false)
      (Transformation|SetRelativeRotation (Variables|Default|GetRightClaw) (Math|Rotator|Lerp(Rotator) (Variables|/Script/Engine.SceneComponent|GetRelativeRotation (Variables|Default|GetLeftClaw)) "60.000000, 0,0.000000" _lerp) false false))))

(event Custom|server_claw
  (CallFunction|FCheckServer))

(event EventBeginPlay
  (|CallParentFunction) ; This node is disabled and will not be called.\nDrag off pins to build functionality.
)

(event Collision|EventActorBeginOverlap
  (params (OtherActor :type Actor%20Object%20Reference))
  (|CallParentFunction OtherActor) ; This node is disabled and will not be called.\nDrag off pins to build functionality.
)

(event EventTick
  (params (DeltaSeconds :type Float%20%28single-precision%29))
  (|CallParentFunction DeltaSeconds) ; This node is disabled and will not be called.\nDrag off pins to build functionality.
)

(fn ConstructionScript
  (|CallParentFunction))

(fn FCheckServer
  (Networking|SwitchHasAuthority
    (:Authority
      (CallFunction|MulticastClaws))
    (:Remote
      (CallFunction|ServerClaw))))