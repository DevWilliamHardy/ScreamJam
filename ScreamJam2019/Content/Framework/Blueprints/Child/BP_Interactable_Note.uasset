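; BP_Interactable_Note is an interactable note that moves up to the interacting character for inspection and returns when used again.
; It caches its world location and rotation on BeginPlay as the resting transform.
; Each interact flips a FlipFlop that plays or reverses the NoteLerp timeline, whose update lerps the actor between that transform and the character's Inspection component, sampled live on every update.
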(event Custom|interact
  (params (CharRef :type Bp%20Char%20Master%20Object%20Reference))
  (bind _inspection (Variables|/Game/Framework/Blueprints/bp_char_master.bp_char_master_C|GetInspection CharRef))
  (Utilities|FlowControl|FlipFlop
    (:A
      (bind _lerp (Timeline|NoteLerp Play)
        (:Update
          (Transformation|SetActorLocationAndRotation (Math|Vector|Lerp(Vector) (Variables|Default|GetBaseLocNote) (Transformation|GetWorldLocation _inspection) _lerp) (Math|Rotator|Lerp(Rotator) (Variables|Default|GetBaseRotNote) (Transformation|GetWorldRotation _inspection) _lerp)))))
    (:B
      (Timeline|NoteLerp Reverse))))

(event Collision|EventActorBeginOverlap
  (params (OtherActor :type Actor%20Object%20Reference))
  (|CallParentFunction OtherActor) ; This node is disabled and will not be called.\nDrag off pins to build functionality.
)

(event EventTick
  (params (DeltaSeconds :type Float%20%28single-precision%29))
  (|CallParentFunction DeltaSeconds) ; This node is disabled and will not be called.\nDrag off pins to build functionality.
)

(event EventBeginPlay
  (Variables|Default|SetBaseLocNote (Transformation|GetActorLocation))
  (Variables|Default|SetBaseRotNote (Transformation|GetActorRotation)))

(fn ConstructionScript
  (|CallParentFunction))