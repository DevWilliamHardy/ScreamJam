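; Single interactable door, child of an interactable base, that swings open and closed on alternate interactions unless locked.
; A timeline lerps the mesh from its BeginPlay rotation to a fixed rotation and reverses to close.
; When the swing finishes, a second timeline ramps the cached patient character's walk speed up, then restores it.
; CineCam toggles the same swing through its own FlipFlop, ignoring the lock.
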(event EventCineCam
  (bind _bp_charpatientref (Variables|Default|GetBP_CharPatientRef))
  (bind _charactermovement (Variables|/Script/Engine.Character|GetCharacterMovement _bp_charpatientref))
  (Utilities|FlowControl|FlipFlop
    (:A
      (bind _lerp (Timeline|Timeline_0 Play)
        (:Update
          (Transformation|SetRelativeRotation (Variables|Default|GetInteractable) (Math|Rotator|Lerp(Rotator) (Variables|Default|GetBaseRotDoor) "0,90.000000, 0" _lerp) false false))
        (:Finished
          (Utilities|IsValid _bp_charpatientref
            (:Is%20Valid
              (bind _output_get (Variables|Default|SetInitialSpeed (Variables|/Script/Engine.CharacterMovementComponent|GetMaxWalkSpeed _charactermovement)))
              (bind _lerp_2 (Timeline|Timeline_1 PlayFromStart)
                (:Update
                  (Variables|/Script/Engine.CharacterMovementComponent|SetMaxWalkSpeed _charactermovement (Math|Float|Lerp _output_get (* _output_get 1.5) _lerp_2)))
                (:Finished
                  (Variables|/Script/Engine.CharacterMovementComponent|SetMaxWalkSpeed _charactermovement (Variables|Default|GetInitialSpeed)))))))))
    (:B
      (Timeline|Timeline_0 Reverse))))

(event Collision|EventActorBeginOverlap
  (params (OtherActor :type Actor%20Object%20Reference))
  (|CallParentFunction OtherActor) ; This node is disabled and will not be called.\nDrag off pins to build functionality.
)

(event EventTick
  (params (DeltaSeconds :type Float%20%28single-precision%29))
  (|CallParentFunction DeltaSeconds) ; This node is disabled and will not be called.\nDrag off pins to build functionality.
)

(event EventBeginPlay
  (|CallParentFunction)
  (Variables|Default|SetBaseRotDoor (Variables|/Script/Engine.SceneComponent|GetRelativeRotation (Variables|Default|GetInteractable))))

(event EventInteract
  (params (CharRef :type Bp%20Char%20Master%20Object%20Reference))
  (bind _asbp_char_patient (Utilities|Casting|CastTobp_char_Patient CharRef)
    (:then
      (Variables|Default|SetBP_CharPatientRef _asbp_char_patient))
    (:CastFailed
      _))
  (if (not (Variables|Default|GetLocked?))
    (Utilities|FlowControl|FlipFlop
      (:A
        (bind _lerp (Timeline|Timeline_0 Play)
          (:Update
            (Transformation|SetRelativeRotation (Variables|Default|GetInteractable) (Math|Rotator|Lerp(Rotator) (Variables|Default|GetBaseRotDoor) "0,90.000000, 0" _lerp) false false))
          (:Finished
            (Utilities|IsValid (Variables|Default|GetBP_CharPatientRef)
              (:Is%20Valid
                (bind _output_get (Variables|Default|SetInitialSpeed (Variables|/Script/Engine.CharacterMovementComponent|GetMaxWalkSpeed (Variables|/Script/Engine.Character|GetCharacterMovement (Variables|Default|GetBP_CharPatientRef)))))
                (bind _lerp_2 (Timeline|Timeline_1 PlayFromStart)
                  (:Update
                    (Variables|/Script/Engine.CharacterMovementComponent|SetMaxWalkSpeed (Variables|/Script/Engine.Character|GetCharacterMovement (Variables|Default|GetBP_CharPatientRef)) (Math|Float|Lerp _output_get (* _output_get 1.5) _lerp_2)))
                  (:Finished
                    (Variables|/Script/Engine.CharacterMovementComponent|SetMaxWalkSpeed (Variables|/Script/Engine.Character|GetCharacterMovement (Variables|Default|GetBP_CharPatientRef)) (Variables|Default|GetInitialSpeed)))))))))
      (:B
        (Timeline|Timeline_0 Reverse)))))

(fn ConstructionScript
  (|CallParentFunction))