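; BP_Interactable_Purse is an interactable purse that opens and closes and holds a coin.
; On BeginPlay it spawns a BP_Interactable_Coin and moves it to the Coin component's location.
; Interact alternates playing and reversing the LerpOpen timeline, which pitches the Interactable component between two rotations.
; When the timeline finishes in either direction, it forwards Interact and the character to the coin if still valid.
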(event EventBeginPlay
  (|CallParentFunction)
  (bind _returnvalue (Game|SpawnActorfromClass "/Game/Framework/Blueprints/Child/BP_Interactable_Coin.BP_Interactable_Coin_C" (Math|Transform|MakeTransform "0, 0, 0") "AlwaysSpawn" 0 0))
  (bind _output_get (Variables|Default|SetCoinRef _returnvalue))
  (Transformation|SetActorLocation _output_get (Transformation|GetWorldLocation (Variables|Default|GetCoin)) false false))

(event Collision|EventActorBeginOverlap
  (params (OtherActor :type Actor%20Object%20Reference))
  (|CallParentFunction OtherActor) ; This node is disabled and will not be called.\nDrag off pins to build functionality.
)

(event EventTick
  (params (DeltaSeconds :type Float%20%28single-precision%29))
  (|CallParentFunction DeltaSeconds) ; This node is disabled and will not be called.\nDrag off pins to build functionality.
)

(event EventInteract
  (params (CharRef :type Bp%20Char%20Master%20Object%20Reference))
  (bind _coinref (Variables|Default|GetCoinRef))
  (Utilities|FlowControl|FlipFlop
    (:A
      (bind _lerp (Timeline|lerpOpen Play)
        (:Update
          (Transformation|SetRelativeRotation (Variables|Default|GetInteractable) (Math|Rotator|Lerp(Rotator) "0, 0,90.000000" "0, 0,20.000000" _lerp) false false))
        (:Finished
          (Utilities|IsValid _coinref
            (:Is%20Valid
              (Default|Interact _coinref CharRef))))))
    (:B
      (Timeline|lerpOpen Reverse))))

(fn ConstructionScript
  (|CallParentFunction))