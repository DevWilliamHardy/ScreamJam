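; Interactable double door that swings both leaves open and closed on alternate Interact calls.
; BeginPlay caches each leaf's starting relative rotation without calling the parent's BeginPlay.
; A FlipFlop plays or reverses one timeline, whose alpha lerps the Interactable and DoubleDoorR components from those cached rotations toward fixed, opposite 90-degree targets.
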(event Collision|EventActorBeginOverlap
  (params (OtherActor :type Actor%20Object%20Reference))
  (|CallParentFunction OtherActor) ; This node is disabled and will not be called.\nDrag off pins to build functionality.
)

(event EventTick
  (params (DeltaSeconds :type Float%20%28single-precision%29))
  (|CallParentFunction DeltaSeconds) ; This node is disabled and will not be called.\nDrag off pins to build functionality.
)

(event EventBeginPlay
  (Variables|Default|SetBaseRotDoor_L (Variables|/Script/Engine.SceneComponent|GetRelativeRotation (Variables|Default|GetInteractable)))
  (Variables|Default|SetBaseRotDoorR (Variables|/Script/Engine.SceneComponent|GetRelativeRotation (Variables|Default|GetDoubleDoor_R))))

(event EventInteract
  (params (CharRef :type Bp%20Char%20Master%20Object%20Reference))
  (Utilities|FlowControl|FlipFlop
    (:A
      (bind _lerp (Timeline|Timeline_0 Play)
        (:Update
          (Transformation|SetRelativeRotation (Variables|Default|GetInteractable) (Math|Rotator|Lerp(Rotator) (Variables|Default|GetBaseRotDoor_L) "0,90.000000, 0" _lerp) false false)
          (Transformation|SetRelativeRotation (Variables|Default|GetDoubleDoor_R) (Math|Rotator|Lerp(Rotator) (Variables|Default|GetBaseRotDoorR) "0,-90.000000,0.000000" _lerp) false false))))
    (:B
      (Timeline|Timeline_0 Reverse))))

(fn ConstructionScript
  (|CallParentFunction))