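; Interactable torch actor that a character picks up through its Interact event.
; Interact stores the character, then plays the Lerp timeline to blend the torch's location and rotation toward the "s_torch" socket on the character's mesh.
; Each update blends from the current transform toward the live socket transform, so the torch follows a moving character.
; When the timeline finishes, the torch snaps and attaches to that socket.
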(event EventBeginPlay
  (|CallParentFunction) ; This node is disabled and will not be called.\nDrag off pins to build functionality.
)

(event Collision|EventActorBeginOverlap
  (params (OtherActor :type Actor%20Object%20Reference))
  (|CallParentFunction OtherActor) ; This node is disabled and will not be called.\nDrag off pins to build functionality.
)

(event EventTick
  (params (DeltaSeconds :type Float%20%28single-precision%29))
  (|CallParentFunction DeltaSeconds) ; This node is disabled and will not be called.\nDrag off pins to build functionality.
)

(event EventInteract
  (params (CharRef :type Bp%20Char%20Master%20Object%20Reference))
  (bind _output_get (Variables|Default|SetCharRef CharRef))
  (bind _lerp (Timeline|lerp PlayFromStart)
    (:Update
      (Transformation|SetActorLocationAndRotation (Math|Vector|Lerp(Vector) (Transformation|GetActorLocation) (Transformation|GetSocketLocation (Variables|/Script/Engine.Character|GetMesh _output_get) "s_torch") _lerp) (Math|Rotator|Lerp(Rotator) (Transformation|GetActorRotation) (Transformation|GetSocketRotation (Variables|/Script/Engine.Character|GetMesh _output_get) "s_torch") _lerp)))
    (:Finished
      (Transformation|AttachComponentToComponent (Variables|/Script/Engine.Character|GetMesh _output_get) "s_torch" "SnapToTarget" "SnapToTarget" "SnapToTarget" true))))

(fn ConstructionScript
  (|CallParentFunction))