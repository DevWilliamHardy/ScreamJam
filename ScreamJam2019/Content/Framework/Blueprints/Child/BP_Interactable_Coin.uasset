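; Coin pickup, a child interactable that a bp_char_Patient collects by interacting with it.
; Interact runs the Coinlerp timeline, lerping the coin from its current location toward the character's live head socket each update, so it homes in on a moving target.
; When the timeline finishes, it increments the character's CoinCount, calls AddWidget for the coin, then destroys itself after a short delay.
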(event EventBeginPlay
  (|CallParentFunction) ; This node is disabled and will not be called.\nDrag off pins to build functionality.
)

(event Collision|EventActorBeginOverlap
  (params (OtherActor :type Actor%20Object%20Reference))
  (|CallParentFunction OtherActor) ; This node is disabled and will not be called.\nDrag off pins to build functionality.
)

(event EventTick
  (params (DeltaSeconds :type Float%20%28single-precision%29))
  (|CallParentFunction DeltaSeconds) ; This node is disabled and will not be called.\nDrag off pins to build functionality.
)

(event EventInteract
  (params (CharRef :type Bp%20Char%20Master%20Object%20Reference))
  (bind _asbp_char_patient (Utilities|Casting|CastTobp_char_Patient CharRef))
  (Variables|Default|SetCharRef _asbp_char_patient)
  (bind _lerp (Timeline|Coinlerp PlayFromStart)
    (:Update
      (Transformation|SetActorLocation self (Math|Vector|Lerp(Vector) (Transformation|GetActorLocation) (Transformation|GetSocketLocation (Variables|/Script/Engine.Character|GetMesh (Variables|Default|GetCharRef)) "head") _lerp) false false))
    (:Finished
      (Variables|/Game/Framework/Blueprints/bp_char_Patient.bp_char_Patient_C|SetCoinCount (Variables|Default|GetCharRef) (+ (Variables|/Game/Framework/Blueprints/bp_char_Patient.bp_char_Patient_C|GetCoinCount (Variables|Default|GetCharRef)) 1))
      (Default|AddWidget (Variables|Default|GetCharRef) "Coin")
      (Utilities|FlowControl|Delay 0.2)
      (Actor|DestroyActor self))))

(fn ConstructionScript
  (|CallParentFunction))