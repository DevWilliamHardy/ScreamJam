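; BP_Interactable_Card is a keycard pickup that grants the patient character card access to readers.
; On Interact, it casts to bp_char_Patient, then a timeline disables collision and lerps the card from its current location to the character.
; When the timeline finishes, it sets the character's Keycard flag, appends its ReaderRef entries to ReaderAvailable and destroys itself.
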(event EventBeginPlay
  (|CallParentFunction) ; This node is disabled and will not be called.\nDrag off pins to build functionality.
)

(event Collision|EventActorBeginOverlap
  (params (OtherActor :type Actor%20Object%20Reference))
  (|CallParentFunction OtherActor) ; This node is disabled and will not be called.\nDrag off pins to build functionality.
)

(event EventInteract
  (params (CharRef :type Bp%20Char%20Master%20Object%20Reference))
  (bind _asbp_char_patient (Utilities|Casting|CastTobp_char_Patient CharRef))
  (bind _output_get (Variables|Default|SetcharRef _asbp_char_patient))
  (bind _lerpcard (Timeline|Timeline_0 Play)
    (:Update
      (Collision|SetCollisionEnabled (Variables|Default|GetInteractable) "NoCollision")
      (Transformation|SetActorLocation (Math|Vector|Lerp(Vector) (Transformation|GetActorLocation) (Transformation|GetActorLocation _output_get) _lerpcard) false false))
    (:Finished
      (Variables|/Game/Framework/Blueprints/bp_char_master.bp_char_master_C|SetKeycard? _output_get true)
      (for _array_element (Variables|Default|GetreaderRef)
        (Utilities|Array|Add (Variables|/Game/Framework/Blueprints/bp_char_master.bp_char_master_C|GetReaderAvailable (Variables|Default|GetcharRef)) _array_element))
      (Actor|DestroyActor self))))

(event EventTick
  (params (DeltaSeconds :type Float%20%28single-precision%29))
  (|CallParentFunction DeltaSeconds) ; This node is disabled and will not be called.\nDrag off pins to build functionality.
)

(fn ConstructionScript
  (|CallParentFunction))