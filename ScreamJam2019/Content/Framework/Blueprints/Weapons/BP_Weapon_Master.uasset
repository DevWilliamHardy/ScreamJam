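; BP_Weapon_Master is a master weapon actor that handles networked melee attacks for the Axe and Bat modes, which share one path.
; The client event passes a cooldown gate, waits briefly, sphere-traces ahead of the character and sends the hit to the server.
; The server applies random-range damage, multiplied for Head bone hits, then multicasts surface-specific impact particles and clears the cooldown after a delay.
; Debug trace drawing and prints remain active.
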(event Custom|Client_StartFireWeapon
  (params (CharRef :type Bp%20Char%20Enemy%20Object%20Reference))
  (bind _returnvalue (Transformation|GetActorLocation CharRef))
  (switch Utilities|FlowControl|Switch|SwitchonE_MeleeMode (Variables|Default|GetWeaponMode)
    (:NewEnumerator1
      _)
    (:NewEnumerator2
      _))
  (Utilities|MAxeFireCD)
  (Utilities|FlowControl|Delay 0.2)
  (Utilities|IsValid CharRef
    (:Is%20Valid
      (bind (_outhit _returnvalue_2) (Collision|SphereTraceByChannel (+ _returnvalue "0, 0,40.000000") (+ (+ _returnvalue (* (Math|Vector|GetForwardVector (Variables|/Script/Engine.Character|GetCapsuleComponent CharRef)) 1.1e+02)) "0, 0,30.000000") 4e+01 "TraceTypeQuery1" false (Utilities|Array|MakeArray CharRef) "ForDuration"))
      (Development|PrintString (Utilities|String|ToString(Boolean) _returnvalue_2))
      (CallFunction|ServerFireShoott _outhit _returnvalue_2))))

(event Custom|Server_FireShoott
  (params (HitResult :type Hit%20Result%20Structure) (Hit :type Boolean))
  (bind (_hitresultout _hitout) (CallFunction|FMeleeInfo HitResult Hit))
  (CallFunction|MulticastFireFX _hitresultout _hitout))

(event Custom|Multicast_FireFX
  (params (HitResult :type Hit%20Result%20Structure) (Hit :type Boolean))
  (CallFunction|FAxeFX Hit HitResult)
  (Utilities|FlowControl|Delay (Variables|Default|GetCooldown))
  (Variables|Default|SetIsWeaponCooldownActive? false))

(event Collision|EventActorBeginOverlap
  (params (OtherActor :type Actor%20Object%20Reference)))

(event EventTick
  (params (DeltaSeconds :type Float%20%28single-precision%29)))

(fn ConstructionScript)

(fn FMeleeInfo
  (params (HitResult :type Hit%20Result%20Structure) (Hit :type Boolean))
  (bind (_bblockinghit _binitialoverlap _time _distance _location _impactpoint _normal _impactnormal _physmat _hitactor _hitcomponent _hitbonename) (Collision|BreakHitResult HitResult))
  (bind _returnvalue (Game|GetInstigatorController))
  (bind _self self)
  (if Hit
    (bind _output_get (Variables|Default|SetDamageDealt (Math|Random|RandomIntegerinRange (Variables|Default|GetHitScanMinDamage) (Variables|Default|GetHitScanMaxDamage))))
    (switch name _hitbonename
      (:Default
        (Game|Damage|ApplyDamage _hitactor (Math|Conversions|ToFloat(Integer) _output_get) _returnvalue _self "/Script/Engine.DamageType"))
      (:head
        (Game|Damage|ApplyDamage _hitactor (Math|Conversions|ToFloat(Integer) (* _output_get (Variables|Default|GetHitScanCriticalDamageMultiplier))) _returnvalue _self "/Script/Engine.DamageType"))))
  (return HitResult Hit))

(fn FAxeFX
  (params (Hit :type Boolean) (HitResult :type Hit%20Result%20Structure%20%28by%20ref%29))
  (bind (_bblockinghit _binitialoverlap _time _distance _location _impactpoint _normal _impactnormal _physmat) (Collision|BreakHitResult HitResult))
  (if Hit
    (bind _returnvalue (Effects|SpawnEmitteratLocation (Utilities|Select :Index (Variables|/Script/Engine.PhysicalMaterial|GetSurfaceType _physmat) :SurfaceType_Default (Variables|HitPS|GetHitDefaultImpactPS) :SurfaceType1 (Variables|HitPS|GetHitBodyPS) :SurfaceType2 (Variables|HitPS|GetHitConcretePS) :SurfaceType3 (Variables|HitPS|GetHitWoodPS) :SurfaceType4 (Variables|HitPS|GetHitWaterPS) :SurfaceType5 (Variables|HitPS|GetHitMetalPS)) _impactpoint (Math|Rotator|MakeRotfromZ _impactnormal)))
    (Development|PrintString (Utilities|GetDisplayName _returnvalue))))