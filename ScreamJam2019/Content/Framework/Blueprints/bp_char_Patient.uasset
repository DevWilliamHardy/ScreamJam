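; Patient player character for a multiplayer, round-based game, handling look and turn animation state, an item popup and winning.
; Each tick it derives a clamped head rotation from control versus actor rotation and passes it to a server event.
; Turn input sets turn-in-place flags while stationary, which remote instances send to the server.
; Winning increments Steam game-instance round and score, lowers the player count, calls Winloss on all PC_MP controllers and destroys the pawn.
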(event Custom|server_Win
  (bind _asgi_mp_steam (Utilities|Casting|CastToGI_MP_Steam (Game|GetGameInstance)))
  (Variables|/Game/Framework/Multiplayer/Blueprints/GI_MP_Steam.GI_MP_Steam_C|SetRound _asgi_mp_steam (+ (Variables|/Game/Framework/Multiplayer/Blueprints/GI_MP_Steam.GI_MP_Steam_C|GetRound _asgi_mp_steam) 1))
  (bind _output_get (Variables|/Game/Framework/Multiplayer/Blueprints/GI_MP_Steam.GI_MP_Steam_C|SetScore _asgi_mp_steam (+ (Variables|/Game/Framework/Multiplayer/Blueprints/GI_MP_Steam.GI_MP_Steam_C|GetScore _asgi_mp_steam) 1)))
  (bind _aspc_mp (Utilities|Casting|CastToPC_MP (Pawn|GetController)))
  (Variables|/Game/Framework/Multiplayer/Blueprints/PC_MP.PC_MP_C|SetScore _aspc_mp _output_get)
  (bind _asgs_ps (Utilities|Casting|CastToGS_PS (Variables|Default|GetPlayerState)))
  (Variables|/Game/Framework/Multiplayer/Blueprints/GS_PS.GS_PS_C|SetPlayernumber _asgs_ps (- (Variables|/Game/Framework/Multiplayer/Blueprints/GS_PS.GS_PS_C|GetPlayernumber _asgs_ps) 1))
  (bind _outactors (Actor|GetAllActorsOfClass "/Game/Framework/Multiplayer/Blueprints/PC_MP.PC_MP_C"))
  (for _array_element _outactors
    (Default|Winloss _array_element))
  (Actor|DestroyActor self))

(event Custom|AddWidget
  (params (Item :type String) (ItemIcon :type Texture%202D%20Object%20Reference))
  (bind _returnvalue (UserInterface|CreateWidget "/Game/Framework/Multiplayer/Widgets/W_AddItem.W_AddItem_C"))
  (bind _output_get (Variables|Default|SetW_AddItemRef _returnvalue))
  (Utilities|IsValid _output_get
    (:Is%20Valid
      (Variables|/Game/Framework/Multiplayer/Widgets/W_AddItem.W_AddItem_C|SetItem _output_get Item)
      (Variables|/Game/Framework/Multiplayer/Widgets/W_AddItem.W_AddItem_C|SetItemIcon (Variables|Default|GetW_AddItemRef) ItemIcon)
      (UserInterface|Viewport|AddtoViewport _output_get 0))))

(event Custom|server_SetTurn
  (params (TurnRight :type Boolean) (TurnLeft :type Boolean))
  (Variables|Default|SetTurnRight TurnRight)
  (Variables|Default|SetTurnLeft TurnLeft))

(event Custom|server_setrot
  (params (HeadRot :type Rotator))
  (Variables|Default|SetHeadRot HeadRot))

(event EventBeginPlay)

(event Collision|EventActorBeginOverlap
  (params (OtherActor :type Actor%20Object%20Reference)))

(event EventTick
  (params (DeltaSeconds :type Float%20%28single-precision%29))
  (CallFunction|FHeadRotation))

(event Input|AxisEvents|InputAxisTurn
  (params (AxisValue :type Float%20%28single-precision%29))
  (Utilities|FlowControl|Sequence
    (:then_0
      (Pawn|Input|AddControllerYawInput AxisValue))
    (:then_1
      (Utilities|MCalcTurninPlace AxisValue))
    (:then_2
      (Networking|SwitchHasAuthority
        (:Remote
          (CallFunction|ServerSetTurn (Variables|Default|GetTurnRight) (Variables|Default|GetTurnLeft)))))))

(fn ConstructionScript
  (|CallParentFunction))

(fn FHeadRotation
  (bind _returnvalue (Transformation|GetActorRotation))
  (bind _returnvalue_2 (Pawn|GetControlRotation :!class /Script/Engine.Pawn))
  (bind _asbp_anim_patient (Utilities|Casting|CastToBP_Anim_Patient (Components|SkeletalMesh|GetAnimInstance (Variables|Character|GetMesh))))
  (Variables|Default|SetAnimRefPatient _asbp_anim_patient)
  (bind _output_get (Variables|Default|SetHeadRot (Math|Rotator|MakeRotator (Math|Float|ClampAngle (* (- (.pitch _returnvalue_2) (.pitch _returnvalue)) -1.0) -45.0 45.0) 0.0 (Math|Float|ClampAngle (- (.yaw _returnvalue_2) (.yaw _returnvalue)) 0.0 1.8e+02))))
  (CallFunction|ServerSetrot _output_get))